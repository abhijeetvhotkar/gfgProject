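; Drivable buggy vehicle that leaves wheel tracks in BP_Snow surfaces.
; Throttle, steering and handbrake inputs feed straight into the vehicle movement component.
; On Tick, after a one-frame-length Delay, each wheel socket that has moved and passes a local-X threshold traces down by AffectRange.
; Snow hits use complex-trace FindCollisionUV on UV channel 1 to pass the hit UV and mesh yaw to SnowHit.
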(event EventTick
  (params (DeltaSeconds :type Float%20%28single-precision%29))
  (bind _mesh (Variables|Character|GetMesh))
  (bind _mesh_2 (Variables|Character|GetMesh))
  (bind _mesh_3 (Variables|Character|GetMesh))
  (bind _mesh_4 (Variables|Character|GetMesh))
  (bind _returnvalue (Transformation|GetSocketLocation _mesh_2 "B_R_wheelJNTSocket"))
  (bind _returnvalue_2 (Transformation|GetSocketLocation _mesh_3 "F_L_wheelJNT"))
  (bind _returnvalue_3 (Transformation|GetSocketLocation _mesh_4 "B_L_wheelJNT"))
  (bind _returnvalue_4 (Transformation|GetSocketLocation _mesh "F_R_wheelJNT"))
  (Utilities|FlowControl|Delay DeltaSeconds)
  (Utilities|FlowControl|Sequence
    (:then_0
      (if (and (Math|Vector|NotEqual(Vector) _returnvalue_2 (Variables|Default|GetFLeftTempLoc) 1.0) (> (.x (.location (Transformation|GetSocketTransform _mesh_3 "F_L_wheelJNT" "RTS_Actor"))) 1e+02))
        (bind _output_get (Variables|Default|SetFLeftTempLoc _returnvalue_2))
        (bind (_outhit _returnvalue_5) (Collision|LineTraceByChannel _output_get (- _output_get (Math|Vector|MakeVector 0.0 0.0 (Variables|Default|GetAffectRange))) "TraceTypeQuery1" true 0 "None"))
        (if _returnvalue_5
          (bind _asbp_snow (Utilities|Casting|CastToBP_Snow (.HitActor (Collision|BreakHitResult _outhit))))
          (Default|SnowHit _asbp_snow (.UV (Class|GameplayStatics|FindCollisionUV _outhit 1)) (.yaw (Transformation|GetWorldRotation (Variables|Character|GetMesh)))))))
    (:then_1
      (if (and (Math|Vector|NotEqual(Vector) _returnvalue_4 (Variables|Default|GetFRightTempLoc) 1.0) (> (.x (.location (Transformation|GetSocketTransform _mesh "F_R_wheelJNT" "RTS_Actor"))) 1e+02))
        (bind _output_get_2 (Variables|Default|SetFRightTempLoc _returnvalue_4))
        (bind (_outhit_2 _returnvalue_6) (Collision|LineTraceByChannel _output_get_2 (- _output_get_2 (Math|Vector|MakeVector 0.0 0.0 (Variables|Default|GetAffectRange))) "TraceTypeQuery1" true 0 "None"))
        (if _returnvalue_6
          (bind _asbp_snow_2 (Utilities|Casting|CastToBP_Snow (.HitActor (Collision|BreakHitResult _outhit_2))))
          (Default|SnowHit _asbp_snow_2 (.UV (Class|GameplayStatics|FindCollisionUV _outhit_2 1)) (.yaw (Transformation|GetWorldRotation (Variables|Character|GetMesh)))))))
    (:then_2
      (if (and (Math|Vector|NotEqual(Vector) _returnvalue_3 (Variables|Default|GetBLeftTempLoc) 1.0) (> (.x (.location (Transformation|GetSocketTransform _mesh_4 "B_L_wheelJNT" "RTS_Actor"))) -2e+02))
        (bind _output_get_3 (Variables|Default|SetBLeftTempLoc _returnvalue_3))
        (bind (_outhit_3 _returnvalue_7) (Collision|LineTraceByChannel _output_get_3 (- _output_get_3 (Math|Vector|MakeVector 0.0 0.0 (Variables|Default|GetAffectRange))) "TraceTypeQuery1" true 0 "None"))
        (if _returnvalue_7
          (bind _asbp_snow_3 (Utilities|Casting|CastToBP_Snow (.HitActor (Collision|BreakHitResult _outhit_3))))
          (Default|SnowHit _asbp_snow_3 (.UV (Class|GameplayStatics|FindCollisionUV _outhit_3 1)) (.yaw (Transformation|GetWorldRotation (Variables|Character|GetMesh)))))))
    (:then_3
      (if (and (Math|Vector|NotEqual(Vector) _returnvalue (Variables|Default|GetBRightTempLoc) 1.0) (> (.x (.location (Transformation|GetSocketTransform _mesh_2 "B_R_wheelJNTSocket" "RTS_Actor"))) -2e+02))
        (bind _output_get_4 (Variables|Default|SetBRightTempLoc _returnvalue))
        (bind (_outhit_4 _returnvalue_8) (Collision|LineTraceByChannel _output_get_4 (- _output_get_4 (Math|Vector|MakeVector 0.0 0.0 (Variables|Default|GetAffectRange))) "TraceTypeQuery1" true 0 "None"))
        (if _returnvalue_8
          (bind _asbp_snow_4 (Utilities|Casting|CastToBP_Snow (.HitActor (Collision|BreakHitResult _outhit_4))))
          (Default|SnowHit _asbp_snow_4 (.UV (Class|GameplayStatics|FindCollisionUV _outhit_4 1)) (.yaw (Transformation|GetWorldRotation (Variables|Character|GetMesh)))))))))

(event Input|ActionEvents|InputActionHandbrake
  (params (Key :type Key%20Structure))
  ;[1 1 1] Controls
  (:Pressed
    (Class|WheeledVehicleMovementComponent|SetHandbrakeInput (Variables|Default|GetVehicleMovement) true))
  (:Released
    (Class|WheeledVehicleMovementComponent|SetHandbrakeInput (Variables|Default|GetVehicleMovement) false)))

(event Input|AxisEvents|InputAxisMoveForward
  (params (AxisValue :type Float%20%28single-precision%29))
  ;[1 1 1] Controls
  (Class|WheeledVehicleMovementComponent|SetThrottleInput (Variables|Default|GetVehicleMovement) AxisValue))

(event Input|AxisEvents|InputAxisMoveRight
  (params (AxisValue :type Float%20%28single-precision%29))
  ;[1 1 1] Controls
  (Class|WheeledVehicleMovementComponent|SetSteeringInput (Variables|Default|GetVehicleMovement) AxisValue))

(fn ConstructionScript)