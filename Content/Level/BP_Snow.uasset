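; BP_Snow is a deformable snow surface that records tire tracks in a render target.
; Construction creates dynamic snow and tire track materials from the depth, strength and up-multiplier settings.
; On BeginPlay it creates a white-cleared render target and feeds it to the snow material as displacement.
; Each SnowHit draws the tire material onto that target at the hit UV, scaled and rotated, so tracks accumulate.
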(event Custom|SnowHit
  (params (UVLoc :type Vector%202D%20Structure) (Rotation :type Float%20%28single-precision%29))
  (bind (_canvas _size _context) (Rendering|BeginDrawCanvastoRenderTarget (Variables|Default|GetSnowDeformTexture)))
  (Canvas|DrawMaterial :self _canvas :RenderMaterial (Variables|Default|GetDynamicTireTrack) :ScreenPosition (.Screen%20Position (CallFunction|SetCanvasMaterialScaleandPosition _size UVLoc (Variables|Default|GetTireScale))) :ScreenSize (.Screen%20Size (CallFunction|SetCanvasMaterialScaleandPosition _size UVLoc (Variables|Default|GetTireScale))) :Rotation (+ (* Rotation -1.0) -9e+01))
  (Rendering|EndDrawCanvastoRenderTarget _context))

(event EventBeginPlay
  (CallFunction|RenderTarget))

(fn ConstructionScript
  (bind _returnvalue (Rendering|Material|CreateDynamicMaterialInstance (Variables|Debug|GetStaticMeshComponent) 0 "/Game/Level/M_Snow.M_Snow" :!class /Script/Engine.PrimitiveComponent))
  (bind _output_get (Variables|Default|SetDynamicSnow _returnvalue))
  (Rendering|Material|SetScalarParameterValue _output_get "SnowOffset" (Variables|Default|GetSnowDepth) :!class /Script/Engine.MaterialInstanceDynamic)
  (bind _returnvalue_2 (Rendering|Material|CreateDynamicMaterialInstance "/Game/Level/M_TireTrack.M_TireTrack" :!class /Script/Engine.KismetMaterialLibrary))
  (bind _output_get_2 (Variables|Default|SetDynamicTireTrack _returnvalue_2))
  (Rendering|Material|SetScalarParameterValue _output_get_2 "StrengthTire" (Variables|Default|GetTireStrength) :!class /Script/Engine.MaterialInstanceDynamic)
  (Rendering|Material|SetScalarParameterValue _output_get_2 "UpMult" (Variables|Default|GetTireUpMult) :!class /Script/Engine.MaterialInstanceDynamic))

(fn RenderTarget
  (bind _returnvalue (Rendering|CreateRenderTarget2D 1024 1024))
  (bind _output_get (Variables|Default|SetSnowDeformTexture _returnvalue))
  (Rendering|ClearRenderTarget2D _output_get "(R=1.000000,G=1.000000,B=1.000000,A=1.000000)")
  (Rendering|Material|SetTextureParameterValue (Variables|Default|GetDynamicSnow) "Displacement" _output_get))